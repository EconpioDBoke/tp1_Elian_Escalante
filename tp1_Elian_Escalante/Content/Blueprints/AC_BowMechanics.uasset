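; AC_BowMechanics is an actor component that gives its owning character a bow and tracks whether it is aiming.
; On BeginPlay it caches the owner as a Character, then spawns BowClass and snaps it to the character mesh at BowSocket.
; AimStar and AimEnd set the IsAiming flag and switch the spawned bow's BowState enum between its two aim-related values.
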(event Custom|AimStar
  (Variables|Default|SetIsAiming true)
  (Variables|/Game/Blueprints/BP_Bow.BP_Bow_C|SetBowState (Variables|Default|GetBowRef) "NewEnumerator1"))

(event Custom|AimEnd
  (Variables|Default|SetIsAiming false)
  (Variables|/Game/Blueprints/BP_Bow.BP_Bow_C|SetBowState (Variables|Default|GetBowRef) "NewEnumerator0"))

(event EventBeginPlay
  (bind _ascharacter (Utilities|Casting|CastToCharacter (Components|GetOwner)))
  (Variables|Default|SetCharacterRef _ascharacter)
  (CallFunction|SpawnBow))

(fn SpawnBow
  (bind _returnvalue (Game|SpawnActorfromClass (Variables|Default|GetBowClass) (Math|Transform|MakeTransform "0, 0, 0" "0, 0, 0" "1.000000,1.000000,1.000000") "Undefined" "MultiplyWithRoot" 0 0))
  (bind _output_get (Variables|Default|SetBowRef _returnvalue))
  (Transformation|AttachComponentToComponent _output_get (Variables|/Script/Engine.Character|GetMesh (Variables|Default|GetCharacterRef)) (Variables|Default|GetBowSocket) "SnapToTarget" "SnapToTarget" "SnapToTarget" true))