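; Arrow projectile actor that stays collision-free until Fire launches it with speed and gravity interpolated from shot strength.
; Fire adds projectile movement at runtime, attaches a Niagara trail and configures the hit effect, disabling fire and smoke below maximum strength.
; Overlapping anything but its instigator removes movement, sticks the arrow, replays the hit effect and pushes physics objects with launch velocity.
; After a delay it clears the trail and sets its lifespan.
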(event OnComponentBeginOverlap(collisionArrow)
  (params (OverlappedComponent :type Primitive%20Component%20Object%20Reference) (OtherActor :type Actor%20Object%20Reference) (OtherComp :type Primitive%20Component%20Object%20Reference) (OtherBodyIndex :type Integer) (bFromSweep :type Boolean) (SweepResult :type Hit%20Result%20Structure%20%28by%20ref%29))
  (bind _hitcomponent (Collision|BreakHitResult SweepResult))
  (if (!= OtherActor (Game|GetInstigator))
    (bind _projectilemovementcomponet (Variables|Default|GetProjectileMovementComponet)
      (:then
        (Components|DestroyComponent _projectilemovementcomponet))
      (:else
        _))
    (Collision|SetCollisionEnabled (Variables|Default|GetcollisionArrow) "NoCollision")
    (Transformation|AttachComponentToComponent _hitcomponent "None" "KeepWorld" "KeepWorld" "KeepWorld" true)
    (Niagara|ResetSystem (Variables|Default|GetHitNiagaraEffect))
    (if (Physics|IsSimulatingPhysics _hitcomponent "None")
      (Physics|AddImpulse _hitcomponent (Variables|Default|GetVelocity) "None" true))
    (Utilities|FlowControl|Delay 1.0)
    (bind _traileffectref (Variables|Default|GetTrailEffectRef)
      (:then
        (Components|DestroyComponent _traileffectref)
        (Actor|SetLifeSpan (Variables|Actor|GetInitialLifeSpan)))
      (:else))))

(event Custom|Fire
  (params (Direction :type Vector) (Stregh :type Float%20%28double-precision%29) (IsIsMaximumStrength :type Boolean))
  (Transformation|SetRelativeRotation (Variables|Default|GetcollisionArrow) "0.000000,90.000000,0.000000" false false)
  (Variables|Default|SetIsMaximumStrength IsIsMaximumStrength)
  (bind _returnvalue (AddComponent|AddProjectileMovementComponent))
  (Variables|Default|SetProjectileMovementComponet _returnvalue)
  (bind _output_get (Variables|/Script/Engine.MovementComponent|SetVelocity _returnvalue (* Direction (Math|Float|Lerp (Variables|Default|GetMinSpeed) (Variables|Default|GetMaxSpeed) Stregh))))
  (Variables|Default|SetVelocity _output_get)
  (Variables|/Script/Engine.ProjectileMovementComponent|SetProjectileGravityScale _returnvalue (Math|Float|Lerp (Variables|Default|GetMaxGravity) (Variables|Default|GetMinGravity) Stregh))
  (bind _returnvalue_2 (Niagara|SpawnSystemAttached (Variables|Default|GetTrailEffect) (Variables|Default|GetArrowEffectLocation) "None" "0, 0, 0" "0, 0, 0" "KeepRelativeOffset" false))
  (Variables|Default|SetTrailEffectRef _returnvalue_2)
  (Collision|SetCollisionEnabled (Variables|Default|GetcollisionArrow) "QueryAndPhysics")
  (CallFunction|DefineParticleHit)
  (Utilities|FlowControl|Delay 0.2))

(event EventBeginPlay
  (Collision|SetCollisionEnabled (Variables|Default|GetcollisionArrow) "NoCollision"))

(fn ConstructionScript)

(fn DefineParticleHit
  (bind _hitniagaraeffect (Variables|Default|GetHitNiagaraEffect))
  (Rendering|SetVisibility _hitniagaraeffect true false)
  (if (not (Variables|Default|GetIsMaximumStrength))
    (Class|NiagaraComponent|SetVariableInt _hitniagaraeffect "User.SpawnCountEmbers" 50)
    (Effects|Components|ParticleSystem|SetEmitterEnable _hitniagaraeffect "Fire" false)
    (Effects|Components|ParticleSystem|SetEmitterEnable _hitniagaraeffect "Smoke" false)))