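; Water actor Blueprint that makes its mesh material adjustable at runtime through an on-screen HUD.
; On BeginPlay it creates a dynamic instance of the static mesh's first material, applies it, and creates a WBP_WaterMatHUD widget that receives that instance.
; Pressing the 1 key toggles the widget on and off the viewport via a FlipFlop.
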(event EventBeginPlay
  (bind _staticmeshcomponent (Variables|Debug|GetStaticMeshComponent))
  (bind _returnvalue (Rendering|Material|CreateDynamicMaterialInstance (Rendering|Material|GetMaterial _staticmeshcomponent 0) "Water_Instance" "None" :!class /Script/Engine.KismetMaterialLibrary))
  (bind _output_get (Variables|Default|SetWater_Instance _returnvalue))
  (Rendering|Material|SetMaterial _staticmeshcomponent 0 _output_get)
  (bind _returnvalue_2 (UserInterface|CreateWidget "/Game/Blueprints/UI/WBP_WaterMatHUD.WBP_WaterMatHUD_C" 0 0))
  (bind _output_get_2 (Variables|Default|SetHUB_Water _returnvalue_2))
  (Variables|/Game/Blueprints/UI/WBP_WaterMatHUD.WBP_WaterMatHUD_C|SetWater_Instance _output_get_2 (Variables|Default|GetWater_Instance)))

(event Collision|EventActorBeginOverlap
  (params (OtherActor :type Actor%20Object%20Reference)))

(event EventTick
  (params (DeltaSeconds :type Float%20%28single-precision%29)))

(event Input|KeyboardEvents|1
  (params (Key :type Key%20Structure :default "None"))
  (:Pressed
    (Utilities|FlowControl|FlipFlop
      (:A
        (UserInterface|Viewport|AddtoViewport (Variables|Default|GetHUB_Water) 0))
      (:B
        (Widget|RemovefromParent (Variables|Default|GetHUB_Water))))))

(fn ConstructionScript)